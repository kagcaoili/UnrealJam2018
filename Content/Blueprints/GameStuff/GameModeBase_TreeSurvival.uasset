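; Game mode for a tree survival game that runs three timed hazard levels in sequence, ending in a debug-print win.
; On BeginPlay it finds the sun, wind spawners and dirt pile spawner, then each level uses looping named-function timers: sun rays, wind from a periodically re-picked random spawner, then bug spawns.
; Delays end each level and chain to the next.
; GameOver shows a menu widget and pauses after a short delay.
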(event `self.ReceiveBeginPlay`
  (`|ExecutionSequence`
    (:`then_0`
      (bind _outactors (`GameplayStatics.GetAllActorsOfClass` "/Game/Blueprints/Actors/Sun.Sun_C"))
      (set `self.SunRef` (`|GetArrayItem` _outactors))
      (bind _outactors_2 (`GameplayStatics.GetAllActorsOfClass` "/Game/Blueprints/Actors/SpawnerObject_Wind.SpawnerObject_Wind_C"))
      (set `self.SpawnerObject_WindRefs` _outactors_2)
      (bind _outactors_3 (`GameplayStatics.GetAllActorsOfClass` "/Game/Blueprints/Actors/SpawnerObject_DirtPile.SpawnerObject_DirtPile_C"))
      (set `self.SpawnerObject_Dirtpile` (`|GetArrayItem` _outactors_3)))
    (:`then_1`
      (`self.Level1`))))

(event `Level1`
  (`KismetSystemLibrary.PrintString` "Level1 Start")
  (bind _returnvalue (`KismetSystemLibrary.K2_SetTimer` (`self.SunRef`) "SunRay" (/ 1.0 (`self.SunRate`)) true))
  (`KismetSystemLibrary.Delay` (`self.LevelDuration`))
  (`KismetSystemLibrary.K2_ClearAndInvalidateTimerHandle` _returnvalue)
  (`KismetSystemLibrary.Delay` (`self.LevelChangeDelay`))
  (`self.Level2`))

(event `WindChange`
  (`KismetSystemLibrary.K2_ClearAndInvalidateTimerHandle` (stale `WindChange` _returnvalue))
  (bind _returnvalue (`KismetSystemLibrary.K2_SetTimer` (`|GetArrayItem` (`self.SpawnerObject_WindRefs`) (`KismetMathLibrary.RandomIntegerInRange` 0 3)) "Spawn" (`self.WindBlowRate`) true)))

(event `EndWind`
  (`KismetSystemLibrary.K2_ClearAndInvalidateTimerHandle` (stale `WindChange` _returnvalue)))

(event `Level2`
  (`KismetSystemLibrary.PrintString` "Level2 Start")
  (`self.WindChange`)
  (bind _returnvalue (`KismetSystemLibrary.K2_SetTimer` null "WindChange" (`self.WindChangeRate`) true))
  (`KismetSystemLibrary.Delay` (`self.LevelDuration`))
  (`KismetSystemLibrary.K2_ClearAndInvalidateTimerHandle` _returnvalue)
  (`self.EndWind`)
  (`KismetSystemLibrary.Delay` (`self.LevelChangeDelay`))
  (`self.Level3`))

(event `Level3`
  (`KismetSystemLibrary.PrintString` "Level3 Start")
  (bind _returnvalue (`KismetSystemLibrary.K2_SetTimer` (`self.SpawnerObject_Dirtpile`) "Spawn" (`self.BugSpawnRate`) true))
  (`KismetSystemLibrary.Delay` (`self.LevelDuration`))
  (`KismetSystemLibrary.K2_ClearAndInvalidateTimerHandle` _returnvalue)
  (`self.Win`))

(event `Win`
  (`KismetSystemLibrary.PrintString` "Winner Winner Chicken Dinner"))

(event `GameOver`
  (`KismetSystemLibrary.Delay` 3.0)
  (`WidgetLayoutLibrary.RemoveAllWidgets`)
  (bind _returnvalue (`|CreateWidget` "/Game/Blueprints/Widgets/MenuGameOver.MenuGameOver_C"))
  (`UserWidget.AddToViewport` _returnvalue 0)
  (`WidgetBlueprintLibrary.SetInputMode_UIOnlyEx` (`GameplayStatics.GetPlayerController` 0) _returnvalue)
  (`GameplayStatics.SetGamePaused` true))

(fn `UserConstructionScript`)