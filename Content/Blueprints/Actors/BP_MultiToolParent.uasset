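; BP_MultiToolParent is a base multi-tool actor that fires projectiles and picks up or drops physics objects.
; PullTrigger calls Fire, which spawns ProjectileClass at the Arrow's transform.
; ItemInteract toggles between a short debug-drawn line trace from the Arrow that grabs simulating components via PhysicsHandle, and releasing them.
; Tick moves the handle target to the Hold location with zero rotation; collision-response changes are left unconnected.
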(event `PullTrigger`
  (`KismetSystemLibrary.PrintString` "TriggerPulled")
  (`self.Fire`))

(event `Fire`
  (`|SpawnActorFromClass` (`self.ProjectileClass`) (`SceneComponent.K2_GetComponentToWorld` (`self.Arrow`)) "Undefined" "OverrideRootScale" null null))

(event `self.ReceiveTick`
  (params (DeltaSeconds :type "Float (single-precision)"))
  (`PhysicsHandleComponent.SetTargetLocationAndRotation` :`self` (`self.PhysicsHandle`) :`NewLocation` (`SceneComponent.K2_GetComponentLocation` (`self.Hold`))))

(event `PickupItem`
  (bind _arrow (`self.Arrow`))
  (bind _returnvalue (`SceneComponent.K2_GetComponentLocation` _arrow))
  (bind (_outhit _returnvalue_2) (`KismetSystemLibrary.LineTraceSingle` :`Start` _returnvalue :`End` (+ _returnvalue (* (`SceneComponent.GetForwardVector` _arrow) 300.0)) :`TraceChannel` "TraceTypeQuery1" :`DrawDebugType` "ForDuration"))
  (if _returnvalue_2
    (bind (_bblockinghit _binitialoverlap _time _distance _location _impactpoint _normal _impactnormal _physmat _hitactor _hitcomponent) (`GameplayStatics.BreakHitResult` _outhit))
    (if (`SceneComponent.IsSimulatingPhysics` _hitcomponent "None")
      (`PhysicsHandleComponent.GrabComponentAtLocation` (`self.PhysicsHandle`) _hitcomponent "None" (`SceneComponent.K2_GetComponentLocation` _hitcomponent))
      (set `self.isHoldingSomething` true)
      (`KismetSystemLibrary.PrintString` "Pickup"))))

(event `ItemInteract`
  (if (`self.isHoldingSomething`)
    (`self.DropItem`)
    (else
      (`self.PickupItem`))))

(event `DropItem`
  (`PhysicsHandleComponent.ReleaseComponent` (`self.PhysicsHandle`))
  (set `self.isHoldingSomething` false)
  (`KismetSystemLibrary.PrintString` "Drop"))

(fn `UserConstructionScript`)