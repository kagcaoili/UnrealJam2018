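; SpawnerObject is an actor that repeatedly spawns a configurable actor class on a looping timer started at BeginPlay.
; The Random flag selects between spawning at the root's transform and spawning at a random point in a ring around the spawner.
; Random placement yaws the whole actor, slides StaticMesh along local X between the inner and outer radii, then spawns at that mesh's world location.
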(event `Spawn`
  (if (`self.Random`)
    (`self.SpawnRandom`)
    (else
      (`self.SpawnNormal`))))

(event `SpawnRandom`
  (`self.K2_SetActorRotation` (`KismetMathLibrary.MakeRotator` 0.0 0.0 (`KismetMathLibrary.RandomFloatInRange` 0.0 360.0)))
  (`SceneComponent.K2_SetRelativeLocation` (`self.StaticMesh`) (`KismetMathLibrary.MakeVector` (`KismetMathLibrary.RandomFloatInRange` (`self.InnerSpawnRadius`) (`self.OuterSpawnRadius`))) false false)
  (`|SpawnActorFromClass` (`self.SpawnActorClass`) (`KismetMathLibrary.MakeTransform` (`SceneComponent.K2_GetComponentLocation` (`self.StaticMesh`))) "Undefined" "OverrideRootScale" null null))

(event `self.ReceiveBeginPlay`
  (`KismetSystemLibrary.K2_SetTimer` null "Spawn" 2.0 true))

(event `SpawnNormal`
  (`|SpawnActorFromClass` (`self.SpawnActorClass`) (`SceneComponent.K2_GetComponentToWorld` (`self.DefaultSceneRoot`)) "Undefined" "OverrideRootScale" null null))

(fn `UserConstructionScript`)