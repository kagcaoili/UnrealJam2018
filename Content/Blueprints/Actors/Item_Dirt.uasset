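; Item_Dirt is a dirt item that feeds soil to a Sapling.
; On overlap it prints the other actor's name and, if that is a Sapling, passes SoilAmount to GainSoil, plays a 2D dirt sound and destroys itself.
; On EndPlay it calls ItemInteract on the player's MultiTool if the tool is holding anything, without checking that the held item is this dirt.
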(event `self.ReceiveActorBeginOverlap`
  (params (OtherActor :type "Actor Object Reference"))
  (`KismetSystemLibrary.PrintString` (`KismetStringLibrary.Concat_StrStr` "Item_Dirt Overlap: " (`KismetSystemLibrary.GetDisplayName` OtherActor)))
  (bind _assapling (cast `/Game/Blueprints/Actors/Sapling` OtherActor))
  (`/Game/Blueprints/Actors/Sapling.GainSoil` _assapling (`self.SoilAmount`))
  (`GameplayStatics.PlaySound2D` "/Game/Sound/Dirt16.Dirt16")
  (`self.K2_DestroyActor`))

(event `self.ReceiveEndPlay`
  (params (EndPlayReason :type "EEndPlayReason Enum" :default "Destroyed"))
  (bind _asplayer (cast `/Game/Blueprints/Actors/Player` (`GameplayStatics.GetPlayerCharacter` 0)))
  (bind _multitoolref (`/Game/Blueprints/Actors/Player.MultiToolRef` _asplayer))
  (if (`/Game/Blueprints/Actors/BP_MultiToolParent.isHoldingSomething` _multitoolref)
    (`/Game/Blueprints/Actors/BP_MultiToolParent.ItemInteract` _multitoolref)))

(fn `UserConstructionScript`
  (`parent.UserConstructionScript`))