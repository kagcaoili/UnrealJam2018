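; Enemy actor that takes damage, deals contact damage to overlapping actors not of its class or subclasses, and dies at zero health.
; AnyDamage flags it as attacked and subtracts health, destroying it when depleted.
; Attack plays a sound and a timeline that moves the mesh along X.
; EndPlay, rather than a death event, spawns the drop item, plus a decal and sound at a downward trace hit.
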(event `self.ReceiveAnyDamage`
  (params (Damage :type "Float (single-precision)") (DamageType :type "DamageType Object Reference") (InstigatedBy :type "Controller Object Reference") (DamageCauser :type "Actor Object Reference"))
  (`|ExecutionSequence`
    (:`then_0`
      (`/Engine/EditorBlueprintResources/StandardMacros.DoOnce` false
        (:`Completed`
          (set `self.isAttacked` true))))
    (:`then_1`
      (bind _output_get (set `self.Health` (- (`self.Health`) Damage)))
      (if (<= _output_get 0.0)
        (`self.K2_DestroyActor`)))))

(event `self.ReceiveEndPlay`
  (params (EndPlayReason :type "EEndPlayReason Enum" :default "Destroyed"))
  (bind _returnvalue (`SceneComponent.K2_GetComponentLocation` (`self.CapsuleComponent`)))
  (`|ExecutionSequence`
    (:`then_0`
      (`|SpawnActorFromClass` (`self.DropItemClass`) (`self.GetTransform`) "Undefined" "OverrideRootScale" null null))
    (:`then_1`
      (bind _outhit (`KismetSystemLibrary.LineTraceSingleForObjects` _returnvalue (+ _returnvalue (`KismetMathLibrary.MakeVector` 0.0 0.0 -100.0)) (`|MakeArray` "ObjectTypeQuery1" :!type "EObjectTypeQuery Enum")))
      (bind (_bblockinghit _binitialoverlap _time _distance _location) (`GameplayStatics.BreakHitResult` _outhit))
      (`GameplayStatics.SpawnDecalAtLocation` (`self.DeathDecal`) (50.0 50.0 1.0) _location (struct))
      (`GameplayStatics.SpawnSoundAtLocation` (`self.DeathSound`) _location))))

(event `Attack`
  (`GameplayStatics.SpawnSoundAttached` (`self.AttackSoundCue`))
  (bind (_direction _bodypositionx) (`Timeline|Timeline_Attack` :!via `PlayFromStart`)
    (:`Update`
      (`SceneComponent.K2_SetRelativeLocation` (`self.StaticMesh`) (`KismetMathLibrary.MakeVector` _bodypositionx) false false))))

(event `self.ReceiveActorBeginOverlap`
  (params (OtherActor :type "Actor Object Reference"))
  (if (not (`KismetMathLibrary.ClassIsChildOf` (`GameplayStatics.GetObjectClass` OtherActor) (`GameplayStatics.GetObjectClass` self)))
    (`GameplayStatics.ApplyDamage` OtherActor (`self.Damage`))))

(fn `UserConstructionScript`)