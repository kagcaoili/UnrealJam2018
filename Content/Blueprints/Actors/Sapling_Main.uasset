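; Sapling actor that tracks its own Health and Water values.
; Any damage lowers Health, prints debug messages with the new value, and destroys the actor once Health reaches zero or below.
; A LoseWater event reduces Water by one per call, with no caller or depletion consequence in this Blueprint.
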(event `self.ReceiveAnyDamage`
  (params (Damage :type "Float (single-precision)") (DamageType :type "DamageType Object Reference") (InstigatedBy :type "Controller Object Reference") (DamageCauser :type "Actor Object Reference"))
  (`KismetSystemLibrary.PrintString` "Sapling took damage")
  (bind _output_get (set `self.Health` (- (`self.Health`) Damage)))
  (`KismetSystemLibrary.PrintString` (`KismetStringLibrary.Conv_DoubleToString` _output_get))
  (if (<= _output_get 0.0)
    (`self.K2_DestroyActor`)))

(event `LoseWater`
  (set `self.Water` (- (`self.Water`) 1.0)))

(fn `UserConstructionScript`)