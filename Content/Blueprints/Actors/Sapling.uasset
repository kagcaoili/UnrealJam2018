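; Sapling is an actor that tracks health plus water and soil meters for a plant in the game.
; Incoming damage lowers Health with debug prints, and the actor destroys itself once Health reaches zero or below.
; Separate events decrement each meter by a fixed step or add a supplied amount, without clamping.
; The meters do not affect Health within this graph, and nothing here calls their events.
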(event `self.ReceiveAnyDamage`
  (params (Damage :type "Float (single-precision)") (DamageType :type "DamageType Object Reference") (InstigatedBy :type "Controller Object Reference") (DamageCauser :type "Actor Object Reference"))
  (`KismetSystemLibrary.PrintString` "Sapling took damage")
  (bind _output_get (set `self.Health` (- (`self.Health`) Damage)))
  (`KismetSystemLibrary.PrintString` (`KismetStringLibrary.Conv_DoubleToString` _output_get))
  (if (<= _output_get 0.0)
    (`self.K2_DestroyActor`)))

(event `LoseWater`
  (set `self.WaterMeter` (- (`self.WaterMeter`) 1.0)))

(event `LoseSoil`
  (set `self.SoilMeter` (- (`self.SoilMeter`) 1.0)))

(event `GainWater`
  (params (Water :type "Float (double-precision)"))
  (set `self.WaterMeter` (+ Water (`self.WaterMeter`))))

(event `GainSoil`
  (params (Soil :type "Float (double-precision)"))
  (set `self.SoilMeter` (+ Soil (`self.SoilMeter`))))

(fn `UserConstructionScript`)