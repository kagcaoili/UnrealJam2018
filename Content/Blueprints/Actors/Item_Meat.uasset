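; Item_Meat is a pickup actor that restores health to the player.
; When another actor overlaps it, it prints a debug message and casts that actor to Player.
; On a successful cast it calls GainHealth with its HealthAmount value, then destroys itself.
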(event `self.ReceiveActorBeginOverlap`
  (params (OtherActor :type "Actor Object Reference"))
  (`KismetSystemLibrary.PrintString` (`KismetStringLibrary.Concat_StrStr` "Item_Meat Overlap: " (`KismetSystemLibrary.GetDisplayName` OtherActor)))
  (bind _asplayer (cast `/Game/Blueprints/Actors/Player` OtherActor))
  (`/Game/Blueprints/Actors/Player.Gain Health` _asplayer (`self.HealthAmount`))
  (`self.K2_DestroyActor`))

(fn `UserConstructionScript`
  (`parent.UserConstructionScript`))