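; DirtPile is an actor that acts as a rising mound from which an enemy spawns.
; On BeginPlay a timeline drives the DirtPile component's relative Z location to raise the mound.
; When the timeline finishes, it spawns an AI pawn of EnemyClass at the actor's location, then destroys itself after a short delay.
; EndPlay spawns an Item_Dirt actor at the pile's transform, whatever the reason play ends.
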(event `self.ReceiveBeginPlay`
  (bind (_direction _newtrack_0) (`Timeline|Timeline_MoundRising` :!via `PlayFromStart`)
    (:`Update`
      (`SceneComponent.K2_SetRelativeLocation` (`self.DirtPile`) (`KismetMathLibrary.MakeVector` 0.0 0.0 _newtrack_0) false false))
    (:`Finished`
      (`AIBlueprintHelperLibrary.SpawnAIFromClass` (`self.EnemyClass`) null (`self.K2_GetActorLocation`))
      (`KismetSystemLibrary.Delay` 2.0)
      (`self.K2_DestroyActor`))))

(event `self.ReceiveEndPlay`
  (params (EndPlayReason :type "EEndPlayReason Enum" :default "Destroyed"))
  (`|SpawnActorFromClass` "/Game/Blueprints/Actors/Item_Dirt.Item_Dirt_C" (`self.GetTransform`) "Undefined" "OverrideRootScale" null null))

(fn `UserConstructionScript`)